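; Interactive book actor that the player reads by stepping into its box collision, which blends the camera to the book and shows an interaction widget.
; While active, keys play or reverse a timeline that turns the page by rotating its mesh and driving a material angle for the arc.
; The construction script builds dynamic materials with the page textures and turn parameters.
; Leaving by key or overlap end blends back to the overlapping actor and removes the widget.
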(event OnComponentBeginOverlap(BoxCollision)
  (params (OverlappedComponent :type Primitive%20Component%20Object%20Reference) (OtherActor :type Actor%20Object%20Reference) (OtherComp :type Primitive%20Component%20Object%20Reference) (OtherBodyIndex :type Integer) (bFromSweep :type Boolean) (SweepResult :type Hit%20Result%20Structure%20%28by%20ref%29))
  (bind _returnvalue (Game|GetPlayerController 0))
  (bind _bookinteractiongui (Variables|Default|GetBookInteractionGUI))
  ;[1 1 1] Box Collision Overlap Event
  (Variables|Default|SetInteractive%20Book true)
  (Variables|Default|SetOverlapped%20Actor OtherActor)
  ;;[1 1 1] Switch Target Camera For Reading Book
  (Utilities|IsValid _returnvalue
    (:Is%20Valid
      (Game|Player|SetViewTargetwithBlend _returnvalue self 1.0 "VTBlend_Linear" 0.0 false)
      (Utilities|FlowControl|Delay 1.0)
      (if (not (UserInterface|Viewport|IsinViewport _bookinteractiongui))
        (if (Variables|Default|GetInteractive%20Book)
          (UserInterface|Viewport|AddtoViewport _bookinteractiongui 0))))))

(event OnComponentEndOverlap(BoxCollision)
  (params (OverlappedComponent :type Primitive%20Component%20Object%20Reference) (OtherActor :type Actor%20Object%20Reference) (OtherComp :type Primitive%20Component%20Object%20Reference) (OtherBodyIndex :type Integer))
  (bind _returnvalue (Game|GetPlayerController 0))
  (bind _bookinteractiongui (Variables|Default|GetBookInteractionGUI))
  ;[1 1 1] Box Collision Overlap Event
  (Variables|Default|SetInteractive%20Book false)
  ;;[1 1 1] Switch Target Camera For Reading Book
  (Utilities|IsValid _returnvalue
    (:Is%20Valid
      (Game|Player|SetViewTargetwithBlend _returnvalue (Variables|Default|GetOverlapped%20Actor) 1.0 "VTBlend_Linear" 0.0 false)
      (Utilities|IsValid _bookinteractiongui
        (:Is%20Valid
          (Widget|RemovefromParent _bookinteractiongui))))))

(event Custom|LeaveInteractiveBook
  (bind _returnvalue (Game|GetPlayerController 0))
  (bind _bookinteractiongui (Variables|Default|GetBookInteractionGUI))
  ;[1 1 1] Box Collision Overlap Event
  (Variables|Default|SetInteractive%20Book false)
  ;;[1 1 1] Switch Target Camera For Reading Book
  (Utilities|IsValid _returnvalue
    (:Is%20Valid
      (Game|Player|SetViewTargetwithBlend _returnvalue (Variables|Default|GetOverlapped%20Actor) 1.0 "VTBlend_Linear" 0.0 false)
      (Utilities|IsValid _bookinteractiongui
        (:Is%20Valid
          (Widget|RemovefromParent _bookinteractiongui))))))

(event EventBeginPlay
  ;[1 1 1] Initial Setting
  (Input|EnableInput (Game|GetPlayerController 0))
  (bind _returnvalue (UserInterface|CreateWidget "/Game/MagicianLabatory/BP/InteractiveBook/BP/WBP_BookInteractionGUI.WBP_BookInteractionGUI_C"))
  (Variables|Default|SetBookInteractionGUI _returnvalue))

(event Input|KeyboardEvents|R
  (params (Key :type Key%20Structure))
  (bind _staticmesh_page (Variables|Default|GetStaticMesh_Page))
  (bind _relativerotation (Variables|/Script/Engine.SceneComponent|GetRelativeRotation _staticmesh_page))
  ;[1 1 1] Input ( Previous Page, Next Page, Leave Interactive Book )
  ;;[1 1 1] Previous
  (:Pressed
    (if (Variables|Default|GetInteractive%20Book)
      ;;[1 1 1] Turning over pages of the book
      (bind (_direction _page_rotate_amount _page_arc) (Timeline|Timeline_0 Reverse)
        (:Update
          (Transformation|SetRelativeRotation _staticmesh_page (Math|Rotator|MakeRotator (* _page_rotate_amount (* (Math|Float|Absolute(Float) (Variables|Default|GetPage%20Rotate%20Amount)) -1.0)) (.pitch _relativerotation) (.yaw _relativerotation)) false false)
          (Rendering|Material|SetScalarParameterValue (Variables|Default|GetPageDynamicMaterial) "Angle" _page_arc :!class /Script/Engine.MaterialInstanceDynamic))))))

(event Input|KeyboardEvents|Y
  (params (Key :type Key%20Structure))
  ;[1 1 1] Input ( Previous Page, Next Page, Leave Interactive Book )
  (:Pressed
    (if (Variables|Default|GetInteractive%20Book)
      (CallFunction|LeaveInteractiveBook))))

(event Input|KeyboardEvents|T
  (params (Key :type Key%20Structure))
  (bind _staticmesh_page (Variables|Default|GetStaticMesh_Page))
  (bind _relativerotation (Variables|/Script/Engine.SceneComponent|GetRelativeRotation _staticmesh_page))
  ;[1 1 1] Input ( Previous Page, Next Page, Leave Interactive Book )
  ;;[1 1 1] Next
  (:Pressed
    (if (Variables|Default|GetInteractive%20Book)
      ;;[1 1 1] Turning over pages of the book
      (bind (_direction _page_rotate_amount _page_arc) (Timeline|Timeline_0 Play)
        (:Update
          (Transformation|SetRelativeRotation _staticmesh_page (Math|Rotator|MakeRotator (* _page_rotate_amount (* (Math|Float|Absolute(Float) (Variables|Default|GetPage%20Rotate%20Amount)) -1.0)) (.pitch _relativerotation) (.yaw _relativerotation)) false false)
          (Rendering|Material|SetScalarParameterValue (Variables|Default|GetPageDynamicMaterial) "Angle" _page_arc :!class /Script/Engine.MaterialInstanceDynamic))))))

(fn ConstructionScript
  ;[1 1 1] Creating Dynamic Materials and Initial Setting
  (bind _returnvalue (Rendering|Material|CreateDynamicMaterialInstance (Variables|Default|GetStaticMesh) 1 "/Game/MagicianLabatory/BP/InteractiveBook/Material/M_BookPage.M_BookPage" "None" :!class /Script/Engine.PrimitiveComponent))
  ;;[1 1 1] Book 1, 4 Pages
  (Rendering|Material|SetTextureParameterValue _returnvalue "BookContent" (Variables|Default|GetBookContent_1and4Pages))
  (bind _returnvalue_2 (Rendering|Material|CreateDynamicMaterialInstance (Variables|Default|GetStaticMesh_Page) 0 "/Game/MagicianLabatory/BP/InteractiveBook/Material/MI_BookPage_Anim.MI_BookPage_Anim" "None" :!class /Script/Engine.PrimitiveComponent))
  (Variables|Default|SetPageDynamicMaterial _returnvalue_2)
  ;;[1 1 1] Book 3 Page
  (Rendering|Material|SetTextureParameterValue (Variables|Default|GetPageDynamicMaterial) "FrontPage" (Variables|Default|GetBookContentFront_Anim_3Page))
  ;;[1 1 1] Book 2 Page
  (Rendering|Material|SetTextureParameterValue (Variables|Default|GetPageDynamicMaterial) "BackPage" (Variables|Default|GetBookContentBack_Anim_2Page))
  (Rendering|Material|SetVectorParameterValue (Variables|Default|GetPageDynamicMaterial) "Position" (Math|Conversions|ToLinearColor(Vector) (+ (Variables|Default|GetPagePosition) (Variables|/Script/Engine.SceneComponent|GetRelativeLocation (Variables|Default|GetDefaultSceneRoot)))) :!class /Script/Engine.MaterialInstanceDynamic)
  (Rendering|Material|SetVectorParameterValue (Variables|Default|GetPageDynamicMaterial) "Axis" (Math|Conversions|ToLinearColor(Vector) (Variables|Default|GetPageAxis)) :!class /Script/Engine.MaterialInstanceDynamic))